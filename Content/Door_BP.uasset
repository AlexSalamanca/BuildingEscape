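; A door actor that swings open and closed when its OpenDoor component fires open and close events.
; It stores its starting rotation on BeginPlay and adds a yaw angle from the Swing timeline to it each update.
; Closing reverses the same timeline, and a timeline event track plays a lock sound at the door's location.
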(event OnClose(OpenDoor)
  (bind _openangle (Timeline|Swing Reverse)
    (:Update
      (Transformation|SetActorRotation (Math|Rotator|CombineRotators (Math|Rotator|MakeRotator 0.0 0.0 _openangle) (Variables|Default|GetInitialRotation))))
    (:SoundTiming
      (Audio|PlaySoundatLocation "/Game/Audio/door-lock.door-lock" (Transformation|GetActorLocation) "0, 0, 0" 1.0 1.0 0.0 0 0 0))))

(event OnOpen(OpenDoor)
  (bind _openangle (Timeline|Swing Play)
    (:Update
      (Transformation|SetActorRotation (Math|Rotator|CombineRotators (Math|Rotator|MakeRotator 0.0 0.0 _openangle) (Variables|Default|GetInitialRotation))))
    (:SoundTiming
      (Audio|PlaySoundatLocation "/Game/Audio/door-lock.door-lock" (Transformation|GetActorLocation) "0, 0, 0" 1.0 1.0 0.0 0 0 0))))

(event EventBeginPlay
  (Variables|Default|SetInitialRotation (Transformation|GetActorRotation)))

(fn ConstructionScript)